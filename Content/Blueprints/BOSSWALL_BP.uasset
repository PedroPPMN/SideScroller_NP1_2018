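; BOSSWALL_BP is a key-gated wall, by its name guarding a boss area, that moves when the player arrives holding a key.
; On box overlap by a BP_CHARACTER, it passes IsHoldingKey to DesactiveWall, which raises the Mid component to a hardcoded relative position if true.
; When any actor ends overlap, it waits briefly, then lowers Mid to its hardcoded lower position without checking the key.
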(event OnComponentBeginOverlap(Box)
  (params (OverlappedComponent :type Primitive%20Component%20Object%20Reference) (OtherActor :type Actor%20Object%20Reference) (OtherComp :type Primitive%20Component%20Object%20Reference) (OtherBodyIndex :type Integer) (bFromSweep :type Boolean) (SweepResult :type Hit%20Result%20Structure%20%28by%20ref%29))
  (bind _asbp_character (Utilities|Casting|CastToBP_CHARACTER OtherActor))
  (bind _output_get (Variables|/Game/2DSideScrollerBP/Blueprints/BP_CHARACTER.BP_CHARACTER_C|SetisHoldingKey _asbp_character (Variables|/Game/2DSideScrollerBP/Blueprints/BP_CHARACTER.BP_CHARACTER_C|GetisHoldingKey _asbp_character)))
  (CallFunction|DesactiveWall _output_get))

(event Custom|DesactiveWall
  (params (MARCELOBOOLEAN :type Boolean))
  (if MARCELOBOOLEAN
    (Components|MoveComponentTo (Variables|Default|Getmid) "3563.000000,80.000000,775.000000" "0, 0, 0" false false 1.0 false)))

(event EventBeginPlay)

(event Collision|EventActorEndOverlap
  (params (OtherActor :type Actor%20Object%20Reference))
  (Utilities|FlowControl|Delay 2.0)
  (Components|MoveComponentTo (Variables|Default|Getmid) "3563.000000,80.000000,645.000000" "0, 0, 0" false false 1.0 false))

(fn ConstructionScript)